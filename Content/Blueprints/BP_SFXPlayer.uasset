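; BP_SFXPlayer is a one-shot sound effect actor that plays a sound and then removes itself.
; The construction script applies its Sound and VolumeMult variables to the Audio component.
; BeginPlay starts playback from StartTime, and the OnAudioFinished event destroys the actor.
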(event OnAudioFinished(Audio)
  (Actor|DestroyActor))

(event EventBeginPlay
  (Audio|Components|Audio|Play (Variables|Default|GetAudio) (Variables|Default|GetStart%20Time)))

(fn ConstructionScript
  (bind _audio (Variables|Default|GetAudio))
  (Audio|Components|Audio|SetSound _audio (Variables|Default|GetSound))
  (Audio|Components|Audio|SetVolumeMultiplier _audio (Variables|Default|GetVolume%20Mult) :!class /Script/Engine.AudioComponent))