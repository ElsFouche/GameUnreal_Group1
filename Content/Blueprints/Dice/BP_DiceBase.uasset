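; Base physics die that reports which face it landed on and plays impact sounds.
; CalculateAndSetNormals aims arrow components along face normals, sampled from LOD 1 mesh data every VertsPerFace vertices.
; Once velocity is near zero, GetDiceResult picks the most vertical arrow by pitch (downward for four-arrow dice, upward otherwise) and returns its index.
; Blocking hits cycle through throttled sounds, with volume and pitch scaled by speed.
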(event OnComponentHit(DiceMesh)
  (params (HitComponent :type Primitive%20Component%20Object%20Reference) (OtherActor :type Actor%20Object%20Reference) (OtherComp :type Primitive%20Component%20Object%20Reference) (NormalImpulse :type Vector :default "0, 0, 0") (Hit :type Hit%20Result%20Structure%20%28by%20ref%29))
  (bind (_bblockinghit _binitialoverlap _time _distance _location) (Collision|BreakHitResult Hit))
  (bind _volumesfx (CallFunction|GetDefaultVolumeSFX))
  (bind _volumesfx_2 (CallFunction|GetDefaultDiceSFX))
  (if _bblockinghit
    (bind _returnvalue (Physics|GetPhysicsLinearVelocity (Variables|Default|GetDiceMesh) "None"))
    ;[0.15 0.15 0.15 0.5] Max sounds per second
    (Utilities|FlowControl|DoOnce false :!label _label
      (:Completed
        (Utilities|FlowControl|Sequence
          (:then_0
            (Utilities|FlowControl|Delay 0.1)
            (goto _label Reset))
          (:then_1
            (Audio|SpawnSoundatLocation (Utilities|Array|Get(acopy) _volumesfx_2 (Variables|Default|GetSoundCounter)) _location "0, 0, 0" (* (/ (Math|Float|Min(Float) (Math|Vector|VectorLength _returnvalue) 1e+03) 7.5e+02) (Math|Random|RandomFloatinRange (* _volumesfx 0.9) _volumesfx)) (Math|Float|Clamp(Float) (/ (Math|Float|Min(Float) (Math|Vector|VectorLength _returnvalue) 1e+03) 7.5e+02) 0.75 1.2) 0.0 0 "/Game/SFX/Dice/SC_Dice.SC_Dice")
            (bind _result (Math|Integer|IncrementInt (Variables|Default|GetSoundCounter))
              (:%20%20
                (Variables|Default|SetSoundCounter (Math|Integer|%(Integer) _result (Utilities|Array|Length _volumesfx_2)))))))))))

(event Custom|CalculateAndSetNormals
  (bind _returnvalue (Transformation|GetActorLocation))
  (bind _arrows (CallFunction|GetArrows))
  (Variables|Default|SetArrowArr _arrows)
  (bind _meshnormals (CallFunction|CalculateNormals))
  (bind (_arrayelement _arrayindex) (Utilities|ForEachLoopReal _meshnormals :!label _label)
    (:LoopBody
      (if (Utilities|Array|IsValidIndex (Variables|Default|GetArrowArr) _arrayindex)
        (Transformation|SetWorldLocationAndRotation (Utilities|Array|Get(acopy) (Variables|Default|GetArrowArr) _arrayindex) _returnvalue (Math|Rotator|FindLookatRotation (Transformation|GetWorldLocation (Utilities|Array|Get(acopy) (Variables|Default|GetArrowArr) _arrayindex)) (+ (* _arrayelement 50) _returnvalue)) false false)
        (Utilities|Array|SetArrayElem (Variables|Default|GetArrowArr) _arrayindex (Utilities|Array|Get(acopy) (Variables|Default|GetArrowArr) _arrayindex) true)
        (Utilities|FlowControl|Delay 0.0)
        (goto _label Continue)))
    (:Completed
      (for _index (range (Utilities|Array|Length (Variables|Default|GetArrowArr)) (- (Utilities|Array|Length _meshnormals) 1))
        (Rendering|SetVisibility (Utilities|Array|Get(acopy) (Variables|Default|GetArrowArr) _index) false false)))))

(event EventBeginPlay
  (bind _arrows (CallFunction|GetArrows))
  (Variables|Default|SetArrowArr _arrows))

(fn ConstructionScript)

(fn GetArrows
  (bind _arrayelement (Utilities|ForEachLoopReal (Actor|GetComponentsByClass "/Script/Engine.ArrowComponent") :!label _label)
    (:LoopBody
      (Utilities|Array|AddUnique (LocalVariables|GetTempArr) _arrayelement)
      (goto _label Continue))
    (:Completed
      (return (LocalVariables|GetTempArr)))))

(fn CalculateNormals
  (bind _vertsperface (Variables|Default|GetVertsPerFace))
  (bind _normals (Class|KismetProceduralMeshLibrary|GetSectionfromStaticMesh (Variables|/Script/Engine.StaticMeshComponent|GetStaticMesh (Variables|Default|GetDiceMesh)) 1))
  (for _index (range 0 (- (/ (Utilities|Array|Length _normals) _vertsperface) 1))
    (Utilities|Array|Add (LocalVariables|GetNormals) (Utilities|Array|Get(acopy) _normals (* _index _vertsperface))))
  (return (LocalVariables|GetNormals)))

(fn CheckResult
  (params (ArrowList :type Array%20of%20Arrow%20Component%20Object%20References))
  (bind _output_get (LocalVariables|SetArrows ArrowList))
  (for _array_element _output_get
    (if (Math|Float|NearlyEqual(Float) (Math|Float|%(Float) (.pitch (Transformation|GetWorldRotation _array_element)) 3.6e+02) (Math|Float|SelectFloat -9e+01 9e+01 (== (Utilities|Array|Length _output_get) 4)) (LocalVariables|GetTolerance))
      (LocalVariables|SetMostUprightArrow _array_element)
      (LocalVariables|SetTolerance (Math|Float|Absolute(Float) (- (Math|Float|%(Float) (.pitch (Transformation|GetWorldRotation _array_element)) 3.6e+02) (Math|Float|SelectFloat -9e+01 9e+01 (== (Utilities|Array|Length _output_get) 4)))))))
  (return (LocalVariables|GetMostUprightArrow) (Utilities|Array|FindItem (LocalVariables|GetArrows) (LocalVariables|GetMostUprightArrow))))

(fn GetDiceResult
  (params (VelocityTolerance :type Float%20%28single-precision%29))
  (if (Math|Vector|VectorIsNearlyZero (Transformation|GetComponentVelocity (Variables|Default|GetDiceMesh)) VelocityTolerance)
    (bind (_resultarrow _arrowindex) (CallFunction|CheckResult (Variables|Default|GetArrowArr)))
    (return _resultarrow _arrowindex true)
    (else
      (return 0 -1 false))))