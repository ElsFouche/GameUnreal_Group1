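; BP_InteractBase is an interactable base Blueprint that shows a widget hint icon while the player is in range, hidden otherwise.
; On range entry it records the eye-to-icon distance as maximum range and starts a looping timer, cleared on exit.
; PlayerInRange fades the WBP_InteractHint text by distance relative to that maximum, with an offset keeping it partly visible, and billboards the icon toward the player's eye position.
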(event Custom|PlayerInRange
  (bind _returnvalue (Game|Player|GetPlayerPawn 0))
  (bind _interacticon (Variables|Default|GetInteractIcon))
  (bind _returnvalue_2 (Transformation|GetActorLocation _returnvalue))
  (bind _baseeyeheight (Variables|/Script/Engine.Pawn|GetBaseEyeHeight _returnvalue))
  (bind (_x _y _z) (Math|Vector|BreakVector _returnvalue_2))
  (bind _returnvalue_3 (+ _z _baseeyeheight))
  (bind _returnvalue_4 (Math|Vector|MakeVector _x _y _returnvalue_3))
  ;[0.15 0.15 0.15 0.5] Set opacity by distance.
  (bind _aswbp_interact_hint (Utilities|Casting|CastToWBP_InteractHint (UserInterface|GetWidget (Variables|Default|GetInteractIcon))))
  (Default|SetTextOpacity _aswbp_interact_hint (Math|Float|Clamp(Float) (+ (- 1.0 (Math|Float|SafeDivide (Math|Float|SafeDivide (Math|Vector|Distance(Vector) _returnvalue_4 (Transformation|GetWorldLocation (Variables|Default|GetInteractIcon))) 1e+02) (Variables|UI|GetInteractRangeMax))) 0.4)))
  ;[0.15 0.15 0.15 0.5] Billboard
  (Transformation|SetWorldRotation _interacticon (Math|Rotator|FindLookatRotation (Transformation|GetWorldLocation _interacticon) _returnvalue_4) false false))

(event EventBeginPlay
  (Rendering|SetVisibility (Variables|Default|GetInteractIcon) false false))

(event EventPlayerEnteredRange
  (bind _returnvalue (Game|Player|GetPlayerPawn 0))
  (bind _returnvalue_2 (Transformation|GetActorLocation _returnvalue))
  (bind (_x _y _z) (Math|Vector|BreakVector _returnvalue_2))
  (Rendering|SetVisibility (Variables|Default|GetInteractIcon) true false)
  (Variables|UI|SetInteractRangeMax (/ (Math|Vector|Distance(Vector) (Math|Vector|MakeVector _x _y (+ _z (Variables|/Script/Engine.Pawn|GetBaseEyeHeight _returnvalue))) (Transformation|GetWorldLocation (Variables|Default|GetInteractIcon))) 1e+02))
  (bind _returnvalue_3 (Utilities|Time|SetTimerbyEvent (EventDispatchers|CreateEvent :!event Custom|PlayerInRange) 0.1 true true))
  (Variables|UI|SetFadeTimer _returnvalue_3))

(event EventPlayerLeftRange
  (Rendering|SetVisibility (Variables|Default|GetInteractIcon) false false)
  (Utilities|Time|ClearandInvalidateTimerbyHandle (Variables|UI|GetFadeTimer)))

(fn ConstructionScript)