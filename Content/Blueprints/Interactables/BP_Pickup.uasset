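; BP_Pickup is an interactable gold pile that reports its coin count to the player when interaction begins.
; Its construction script runs the parent's, then picks one of three pile meshes by comparing Coins against two thresholds.
; On interaction it checks that the player character implements BPI_Interact, then sends it a Gold item data struct through SendToPlayerMessage.
; The graph shown does not destroy or hide the pickup afterwards.
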(event EventPlayerBeganInteract
  (bind _returnvalue (Game|GetPlayerCharacter 0))
  (if (Utilities|DoesObjectImplementInterface _returnvalue "/Game/Blueprints/Interfaces/BPI_Interact.BPI_Interact_C")
    (Class|BPIInteract|SendtoPlayer(Message) _returnvalue (Utilities|Struct|MakeF_ItemData "Gold" "(Normal=(TintColor=(SpecifiedColor=(R=1.000000,G=1.000000,B=1.000000,A=1.000000),ColorUseRule=UseColor_Specified),DrawAs=Image,Tiling=NoTile,Mirroring=NoMirror,ImageType=NoImage,ImageSize=(X=32.000000,Y=32.000000),Margin=(Left=0.000000,Top=0.000000,Right=0.000000,Bottom=0.000000),ResourceObject=None,OutlineSettings=(CornerRadii=(X=0.000000,Y=0.000000,Z=0.000000,W=0.000000),Color=(SpecifiedColor=(R=0.000000,G=0.000000,B=0.000000,A=0.000000),ColorUseRule=UseColor_Specified),Width=0.000000,RoundingType=HalfHeightRadius,bUseBrushTransparency=False),UVRegion=(Min=(X=0.000000,Y=0.000000),Max=(X=0.000000,Y=0.000000),bIsValid=False),bIsDynamicallyLoaded=False,ResourceName=\"\"),Hovered=(TintColor=(SpecifiedColor=(R=1.000000,G=1.000000,B=1.000000,A=1.000000),ColorUseRule=UseColor_Specified),DrawAs=Image,Tiling=NoTile,Mirroring=NoMirror,ImageType=NoImage,ImageSize=(X=32.000000,Y=32.000000),Margin=(Left=0.000000,Top=0.000000,Right=0.000000,Bottom=0.000000),ResourceObject=None,OutlineSettings=(CornerRadii=(X=0.000000,Y=0.000000,Z=0.000000,W=0.000000),Color=(SpecifiedColor=(R=0.000000,G=0.000000,B=0.000000,A=0.000000),ColorUseRule=UseColor_Specified),Width=0.000000,RoundingType=HalfHeightRadius,bUseBrushTransparency=False),UVRegion=(Min=(X=0.000000,Y=0.000000),Max=(X=0.000000,Y=0.000000),bIsValid=False),bIsDynamicallyLoaded=False,ResourceName=\"\"),Pressed=(TintColor=(SpecifiedColor=(R=1.000000,G=1.000000,B=1.000000,A=1.000000),ColorUseRule=UseColor_Specified),DrawAs=Image,Tiling=NoTile,Mirroring=NoMirror,ImageType=NoImage,ImageSize=(X=32.000000,Y=32.000000),Margin=(Left=0.000000,Top=0.000000,Right=0.000000,Bottom=0.000000),ResourceObject=None,OutlineSettings=(CornerRadii=(X=0.000000,Y=0.000000,Z=0.000000,W=0.000000),Color=(SpecifiedColor=(R=0.000000,G=0.000000,B=0.000000,A=0.000000),ColorUseRule=UseColor_Specified),Width=0.000000,RoundingType=HalfHeightRadius,bUseBrushTransparency=False),UVRegion=(Min=(X=0.000000,Y=0.000000),Max=(X=0.000000,Y=0.000000),bIsValid=False),bIsDynamicallyLoaded=False,ResourceName=\"\"),Disabled=(TintColor=(SpecifiedColor=(R=1.000000,G=1.000000,B=1.000000,A=1.000000),ColorUseRule=UseColor_Specified),DrawAs=NoDrawType,Tiling=NoTile,Mirroring=NoMirror,ImageType=NoImage,ImageSize=(X=0.000000,Y=0.000000),Margin=(Left=0.000000,Top=0.000000,Right=0.000000,Bottom=0.000000),ResourceObject=None,OutlineSettings=(CornerRadii=(X=0.000000,Y=0.000000,Z=0.000000,W=0.000000),Color=(SpecifiedColor=(R=0.000000,G=0.000000,B=0.000000,A=0.000000),ColorUseRule=UseColor_Specified),Width=0.000000,RoundingType=HalfHeightRadius,bUseBrushTransparency=False),UVRegion=(Min=(X=0.000000,Y=0.000000),Max=(X=0.000000,Y=0.000000),bIsValid=False),bIsDynamicallyLoaded=False,ResourceName=\"\"),NormalForeground=(SpecifiedColor=(R=1.000000,G=0.000000,B=1.000000,A=1.000000),ColorUseRule=UseColor_Foreground),HoveredForeground=(SpecifiedColor=(R=1.000000,G=0.000000,B=1.000000,A=1.000000),ColorUseRule=UseColor_Foreground),PressedForeground=(SpecifiedColor=(R=1.000000,G=0.000000,B=1.000000,A=1.000000),ColorUseRule=UseColor_Foreground),DisabledForeground=(SpecifiedColor=(R=1.000000,G=0.000000,B=1.000000,A=1.000000),ColorUseRule=UseColor_Foreground),NormalPadding=(Left=0.000000,Top=0.000000,Right=0.000000,Bottom=0.000000),PressedPadding=(Left=0.000000,Top=0.000000,Right=0.000000,Bottom=0.000000),PressedSlateSound=(ResourceObject=None),ClickedSlateSound=(ResourceObject=None),HoveredSlateSound=(ResourceObject=None))" 0 1 (Variables|Default|GetCoins)))))

(fn ConstructionScript
  (|CallParentFunction)
  (if (Math|Integer|InRange(Integer) (Variables|Default|GetCoins) 0 (Variables|Default|Get1-2%20Change) true false)
    (Components|StaticMesh|SetStaticMesh (Variables|Default|GetStaticMesh) (Variables|Default|GetPile1Mesh))
    (elif (Math|Integer|InRange(Integer) (Variables|Default|GetCoins) (Variables|Default|Get1-2%20Change) (Variables|Default|Get2-3%20Change) true false)
      (Components|StaticMesh|SetStaticMesh (Variables|Default|GetStaticMesh) (Variables|Default|GetPile2Mesh))
      (else
        (Components|StaticMesh|SetStaticMesh (Variables|Default|GetStaticMesh) (Variables|Default|GetPile3Mesh))))))