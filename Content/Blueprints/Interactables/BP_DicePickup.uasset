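; BP_DicePickup is an interactable world pickup that gives the player a die of a configured shape.
; The construction script sets the static mesh to match the DiceType, from D4 to D20.
; On interaction, it sends a single-count dice item to the player character through BPI_Interact, spawns a BP_SFXPlayer actor for the pickup sound, then destroys itself.
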(event EventPlayerBeganInteract
  (bind _returnvalue (Game|GetPlayerCharacter 0))
  (if (Utilities|DoesObjectImplementInterface _returnvalue "/Game/Blueprints/Interfaces/BPI_Interact.BPI_Interact_C")
    (Class|BPIInteract|SendtoPlayer(Message) _returnvalue (Utilities|Struct|MakeF_ItemData "Dice" "(Normal=(TintColor=(SpecifiedColor=(R=1.000000,G=1.000000,B=1.000000,A=1.000000),ColorUseRule=UseColor_Specified),DrawAs=Image,Tiling=NoTile,Mirroring=NoMirror,ImageType=NoImage,ImageSize=(X=32.000000,Y=32.000000),Margin=(Left=0.000000,Top=0.000000,Right=0.000000,Bottom=0.000000),ResourceObject=None,OutlineSettings=(CornerRadii=(X=0.000000,Y=0.000000,Z=0.000000,W=0.000000),Color=(SpecifiedColor=(R=0.000000,G=0.000000,B=0.000000,A=0.000000),ColorUseRule=UseColor_Specified),Width=0.000000,RoundingType=HalfHeightRadius,bUseBrushTransparency=False),UVRegion=(Min=(X=0.000000,Y=0.000000),Max=(X=0.000000,Y=0.000000),bIsValid=False),bIsDynamicallyLoaded=False,ResourceName=\"\"),Hovered=(TintColor=(SpecifiedColor=(R=1.000000,G=1.000000,B=1.000000,A=1.000000),ColorUseRule=UseColor_Specified),DrawAs=Image,Tiling=NoTile,Mirroring=NoMirror,ImageType=NoImage,ImageSize=(X=32.000000,Y=32.000000),Margin=(Left=0.000000,Top=0.000000,Right=0.000000,Bottom=0.000000),ResourceObject=None,OutlineSettings=(CornerRadii=(X=0.000000,Y=0.000000,Z=0.000000,W=0.000000),Color=(SpecifiedColor=(R=0.000000,G=0.000000,B=0.000000,A=0.000000),ColorUseRule=UseColor_Specified),Width=0.000000,RoundingType=HalfHeightRadius,bUseBrushTransparency=False),UVRegion=(Min=(X=0.000000,Y=0.000000),Max=(X=0.000000,Y=0.000000),bIsValid=False),bIsDynamicallyLoaded=False,ResourceName=\"\"),Pressed=(TintColor=(SpecifiedColor=(R=1.000000,G=1.000000,B=1.000000,A=1.000000),ColorUseRule=UseColor_Specified),DrawAs=Image,Tiling=NoTile,Mirroring=NoMirror,ImageType=NoImage,ImageSize=(X=32.000000,Y=32.000000),Margin=(Left=0.000000,Top=0.000000,Right=0.000000,Bottom=0.000000),ResourceObject=None,OutlineSettings=(CornerRadii=(X=0.000000,Y=0.000000,Z=0.000000,W=0.000000),Color=(SpecifiedColor=(R=0.000000,G=0.000000,B=0.000000,A=0.000000),ColorUseRule=UseColor_Specified),Width=0.000000,RoundingType=HalfHeightRadius,bUseBrushTransparency=False),UVRegion=(Min=(X=0.000000,Y=0.000000),Max=(X=0.000000,Y=0.000000),bIsValid=False),bIsDynamicallyLoaded=False,ResourceName=\"\"),Disabled=(TintColor=(SpecifiedColor=(R=1.000000,G=1.000000,B=1.000000,A=1.000000),ColorUseRule=UseColor_Specified),DrawAs=NoDrawType,Tiling=NoTile,Mirroring=NoMirror,ImageType=NoImage,ImageSize=(X=0.000000,Y=0.000000),Margin=(Left=0.000000,Top=0.000000,Right=0.000000,Bottom=0.000000),ResourceObject=None,OutlineSettings=(CornerRadii=(X=0.000000,Y=0.000000,Z=0.000000,W=0.000000),Color=(SpecifiedColor=(R=0.000000,G=0.000000,B=0.000000,A=0.000000),ColorUseRule=UseColor_Specified),Width=0.000000,RoundingType=HalfHeightRadius,bUseBrushTransparency=False),UVRegion=(Min=(X=0.000000,Y=0.000000),Max=(X=0.000000,Y=0.000000),bIsValid=False),bIsDynamicallyLoaded=False,ResourceName=\"\"),NormalForeground=(SpecifiedColor=(R=1.000000,G=0.000000,B=1.000000,A=1.000000),ColorUseRule=UseColor_Foreground),HoveredForeground=(SpecifiedColor=(R=1.000000,G=0.000000,B=1.000000,A=1.000000),ColorUseRule=UseColor_Foreground),PressedForeground=(SpecifiedColor=(R=1.000000,G=0.000000,B=1.000000,A=1.000000),ColorUseRule=UseColor_Foreground),DisabledForeground=(SpecifiedColor=(R=1.000000,G=0.000000,B=1.000000,A=1.000000),ColorUseRule=UseColor_Foreground),NormalPadding=(Left=0.000000,Top=0.000000,Right=0.000000,Bottom=0.000000),PressedPadding=(Left=0.000000,Top=0.000000,Right=0.000000,Bottom=0.000000),PressedSlateSound=(ResourceObject=None),ClickedSlateSound=(ResourceObject=None),HoveredSlateSound=(ResourceObject=None))" 0 0 1 (Variables|Default|GetDiceType)))
    (Game|SpawnActorfromClass "/Game/Blueprints/BP_SFXPlayer.BP_SFXPlayer_C" (Transformation|GetActorTransform) "Undefined" "MultiplyWithRoot" 0 "/Game/SFX/SFX_DicePickup.SFX_DicePickup" 1.0 0.0 0)
    (Actor|DestroyActor)))

(fn ConstructionScript
  (bind _staticmesh (Variables|Default|GetStaticMesh))
  (|CallParentFunction)
  (switch Utilities|FlowControl|Switch|SwitchonE_DiceShapes (Variables|Default|GetDiceType)
    (:NewEnumerator0
      (Components|StaticMesh|SetStaticMesh _staticmesh 0))
    (:NewEnumerator1
      (Components|StaticMesh|SetStaticMesh _staticmesh "/Game/Models/Props/prp_D4.prp_D4"))
    (:NewEnumerator2
      (Components|StaticMesh|SetStaticMesh _staticmesh "/Game/Models/Props/prp_D6.prp_D6"))
    (:NewEnumerator3
      (Components|StaticMesh|SetStaticMesh _staticmesh "/Game/Models/Props/prp_D8.prp_D8"))
    (:NewEnumerator4
      (Components|StaticMesh|SetStaticMesh _staticmesh "/Game/Models/Props/prp_D10.prp_D10"))
    (:NewEnumerator5
      (Components|StaticMesh|SetStaticMesh _staticmesh "/Game/Models/Props/prp_D12.prp_D12"))
    (:NewEnumerator6
      (Components|StaticMesh|SetStaticMesh _staticmesh "/Game/Models/Props/prp_D20.prp_D20"))))