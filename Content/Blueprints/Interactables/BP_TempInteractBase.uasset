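; BP_TempInteractBase is a temporary-named base interactable whose mesh is set from ItemMesh in the Construction Script.
; Its Interact event, when Inspect is enabled, spawns a BP_InspectItem at a far-off location and passes it the character, mesh, name, description, rotation and scale.
; BeginPlay calls Interact on the player's BP_FirstPersonCharacter, so inspection fires as soon as the actor begins play.
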(event EventInteract
  (params (Character :type BP%20First%20Person%20Character%20Object%20Reference))
  (if (Variables|Default|GetInspect?)
    (bind _returnvalue (Game|SpawnActorfromClass "/Game/Blueprints/Interactables/BP_InspectItem.BP_InspectItem_C" (Math|Transform|MakeTransform "10000000.000000,0.000000,0.000000") "Undefined" "MultiplyWithRoot" 0 0))
    (Default|SetInspectRotation _returnvalue (Variables|Default|GetItemInspectRotation))
    (Default|SetInspectScale _returnvalue (Variables|Default|GetItemInspectScale))
    (Class|BPIInteractable|Inspect(Message) _returnvalue Character (Variables|/Script/Engine.StaticMeshComponent|GetStaticMesh (Variables|Default|GetStaticMesh)) (Variables|Default|GetItemName) (Variables|Default|GetItemDescription))))

(event EventBeginPlay
  (bind _asbp_first_person_character (Utilities|Casting|CastToBP_FirstPersonCharacter (Game|GetPlayerCharacter 0)))
  (CallFunction|Interact _asbp_first_person_character))

(fn ConstructionScript
  (Components|StaticMesh|SetStaticMesh (Variables|Default|GetStaticMesh) (Variables|Default|GetItemMesh)))