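; BP_Container is an interactable loot container that opens a shared container UI, optionally behind a skill-check lock.
; On interact it puts the player in UI mode, then either sends the player a lockpick attempt with its DC and prior-attempt flag or fills the game mode's container widget with its items.
; A successful unlock result clears the lock and opens the menu.
; Items the player takes are removed by slot index.
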(event EventBeginPlay
  (|CallParentFunction) ; This node is disabled and will not be called.\nDrag off pins to build functionality.
)

(event EventPlayerBeganInteract
  (Class|BPIUI|SetPlayertoUIMode(Message) (Game|GetPlayerCharacter 0))
  (if (Variables|Container|GetbIsLocked)
    (Class|BPIInteract|TryOpenLock(Message) (Game|GetPlayerCharacter 0) (Variables|Container|GetLockDC) self (Variables|Container|GetbHasAttempted))
    (else
      ;[0.15 0.15 0.15 0.5] Establish reference to existing container UI
      (Variables|UI|GetContainerMenu
        (:then
          _)
        (:else
          (bind _containermenu (Class|BPIInteract|GetContainerWidget(Message) (Game|GetGameMode)))
          (Variables|UI|SetContainerMenu _containermenu)))
      (Default|SetContainerName (Variables|UI|GetContainerMenu) (Variables|Container|GetContainerName))
      (Default|SetOwningContainer (Variables|UI|GetContainerMenu) self)
      ;[0.15 0.15 0.15 0.5] Send new item(s) to widget
      (for (_array_element _array_index) (Variables|Container|GetItems)
        (Default|UpdateItems (Variables|UI|GetContainerMenu) _array_index (Utilities|String|StringToName (Utilities|String|EnumtoString (.itemtype _array_element))) (.count _array_element)))
      ;[0.15 0.15 0.15 0.5] Set Widget Visibility & Focus
      (Widget|SetVisibility (Variables|UI|GetContainerMenu) "Visible")
      (Widget|SetFocus (Variables|UI|GetContainerMenu))
      (Input|SetInputModeUIOnly (Game|GetPlayerController 0) (Variables|UI|GetContainerMenu) "LockAlways" false))))

(event EventPlayerObtainedItem
  (params (ItemSlot :type Integer))
  (bind _items (Variables|Container|GetItems))
  (if (Utilities|Array|IsValidIndex _items ItemSlot)
    (Utilities|Array|RemoveIndex _items ItemSlot)))

(event EventUnlockResult
  (params (bSuccess :type Boolean))
  (if bSuccess
    (Variables|Container|SetbIsLocked false)
    ;[0.15 0.15 0.15 0.5] Establish reference to existing container UI
    (Variables|UI|GetContainerMenu
      (:then
        _)
      (:else
        (bind _containermenu (Class|BPIInteract|GetContainerWidget(Message) (Game|GetGameMode)))
        (Variables|UI|SetContainerMenu _containermenu)))
    (Default|SetContainerName (Variables|UI|GetContainerMenu) (Variables|Container|GetContainerName))
    (Default|SetOwningContainer (Variables|UI|GetContainerMenu) self)
    ;[0.15 0.15 0.15 0.5] Send new item(s) to widget
    (for (_array_element _array_index) (Variables|Container|GetItems)
      (Default|UpdateItems (Variables|UI|GetContainerMenu) _array_index (Utilities|String|StringToName (Utilities|String|EnumtoString (.itemtype _array_element))) (.count _array_element)))
    ;[0.15 0.15 0.15 0.5] Set Widget Visibility & Focus
    (Widget|SetVisibility (Variables|UI|GetContainerMenu) "Visible")
    (Widget|SetFocus (Variables|UI|GetContainerMenu))
    (Input|SetInputModeUIOnly (Game|GetPlayerController 0) (Variables|UI|GetContainerMenu) "LockAlways" false)
    (else
      (Variables|Container|SetbHasAttempted true))))

(fn ConstructionScript
  (|CallParentFunction))

(fn UnlockResult0
  (return))