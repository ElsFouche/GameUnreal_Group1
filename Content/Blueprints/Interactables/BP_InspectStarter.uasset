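; BP_InspectStarter is a one-use interactable item that opens an inspection view for its configurable mesh, name and description.
; While the player is in range, a looping timer billboards the InteractIcon widget toward eye height and fades its text by distance, normalized to the entry distance.
; Interacting spawns BP_ItemInspection at a fixed remote location, passes it the item data, updates the character's inspiration, then destroys this actor next tick.
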(event Custom|PlayerInRange
  (bind _returnvalue (Game|Player|GetPlayerPawn 0))
  (bind _interacticon (Variables|Default|GetInteractIcon))
  (bind _returnvalue_2 (Transformation|GetActorLocation _returnvalue))
  (bind _baseeyeheight (Variables|/Script/Engine.Pawn|GetBaseEyeHeight _returnvalue))
  (bind (_x _y _z) (Math|Vector|BreakVector _returnvalue_2))
  (bind _returnvalue_3 (+ _z _baseeyeheight))
  (bind _returnvalue_4 (Math|Vector|MakeVector _x _y _returnvalue_3))
  ;[0.15 0.15 0.15 0.5] Set opacity by distance.
  (bind _aswbp_interact_hint (Utilities|Casting|CastToWBP_InteractHint (UserInterface|GetWidget (Variables|Default|GetInteractIcon))))
  (Default|SetTextOpacity _aswbp_interact_hint (Math|Float|Clamp(Float) (+ (- 1.0 (Math|Float|SafeDivide (Math|Float|SafeDivide (Math|Vector|Distance(Vector) _returnvalue_4 (Transformation|GetWorldLocation (Variables|Default|GetInteractIcon))) 1e+02) (Variables|Default|GetInteractRangeMax))) 0.4)))
  ;[0.15 0.15 0.15 0.5] Billboard
  (Transformation|SetWorldRotation _interacticon (Math|Rotator|FindLookatRotation (Transformation|GetWorldLocation _interacticon) _returnvalue_4) false false))

(event EventInteract
  (params (Character :type BP%20First%20Person%20Character%20Object%20Reference))
  (bind _returnvalue (Game|SpawnActorfromClass "/Game/Blueprints/Interactables/BP_ItemInspection.BP_ItemInspection_C" (Math|Transform|MakeTransform "1000.000000,-1000.000000,-3500.000000" "0.000000,0.000000,0.000000") "AlwaysSpawn" "MultiplyWithRoot" 0 0))
  (Default|SetInspectRotation _returnvalue (Variables|Default|GetItemInspectRotation))
  (Default|SetInspectScale _returnvalue (Variables|Default|GetItemInspectScale))
  (Class|BPIInteractable|Inspect(Message) _returnvalue Character (Variables|/Script/Engine.StaticMeshComponent|GetStaticMesh (Variables|Default|GetStaticMesh)) (Variables|Default|GetItemName) (Variables|Default|GetItemDescription))
  (bind _asbp_first_person_character (Utilities|Casting|CastToBP_FirstPersonCharacter (Game|Player|GetPlayerPawn 0)))
  (Class|BPIUI|UpdateInspiration(Message) _asbp_first_person_character 1)
  (Utilities|FlowControl|DelayUntilNextTick)
  (Actor|DestroyActor))

(event EventPlayerEnteredRange
  (bind _returnvalue (Game|Player|GetPlayerPawn 0))
  (bind _returnvalue_2 (Transformation|GetActorLocation _returnvalue))
  (bind (_x _y _z) (Math|Vector|BreakVector _returnvalue_2))
  (Rendering|SetVisibility (Variables|Default|GetInteractIcon) true false)
  (Variables|Default|SetInteractRangeMax (/ (Math|Vector|Distance(Vector) (Math|Vector|MakeVector _x _y (+ _z (Variables|/Script/Engine.Pawn|GetBaseEyeHeight _returnvalue))) (Transformation|GetWorldLocation (Variables|Default|GetInteractIcon))) 1e+02))
  (bind _returnvalue_3 (Utilities|Time|SetTimerbyEvent (EventDispatchers|CreateEvent :!event Custom|PlayerInRange) 0.1 true true))
  (Variables|Default|SetFadeTimer _returnvalue_3))

(event EventPlayerLeftRange
  (Rendering|SetVisibility (Variables|Default|GetInteractIcon) false false)
  (Utilities|Time|ClearandInvalidateTimerbyHandle (Variables|Default|GetFadeTimer)))

(event EventPlayerBeganInteract
  (bind _asbp_first_person_character (Utilities|Casting|CastToBP_FirstPersonCharacter (Game|Player|GetPlayerPawn 0)))
  (Class|BPIInteractable|Interact(Message) self _asbp_first_person_character))

(event EventBeginPlay
  (Rendering|SetVisibility (Variables|Default|GetInteractIcon) false false))

(fn ConstructionScript
  (Components|StaticMesh|SetStaticMesh (Variables|Default|GetStaticMesh) (Variables|Default|GetItemMesh)))

(fn GetContainerWidget
  (return 0))