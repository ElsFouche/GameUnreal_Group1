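; Temporary item-inspection actor that displays a given mesh with a name/description widget and updates the character's inspiration message.
; Inspect moves input from the character to this actor; IA_Interact returns it, removes the widget and destroys the actor.
; Left-drag or IA_Move rotates the mesh, the wheel zooms by clamping SceneCaptureComponent2D FOV, and right-click resets both.
; Callers can set starting rotation and scale; construction caches default FOV and positions InteractIcon above the mesh.
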(event Custom|Set%20Inspect%20Scale
  (params (Item%20Scale :type Vector))
  (bind _item (Variables|Default|GetItem))
  (bind _returnvalue (Transformation|GetWorldTransform _item))
  ;[0.15 0.15 0.15 0.5] Set Inspection Scale Dynamically
  (Transformation|SetWorldTransform _item (Math|Transform|MakeTransform (.location _returnvalue) (.rotation _returnvalue) Item%20Scale) false false))

(event Custom|Set%20Inspect%20Rotation
  (params (Item%20Rotation :type Rotator))
  (bind _item (Variables|Default|GetItem))
  (bind _returnvalue (Transformation|GetWorldTransform _item))
  ;[0.15 0.15 0.15 0.5] Set Inspection Rotation Dynamically
  (bind _output_get (Variables|Default|SetInitial%20Rotation Item%20Rotation))
  (Transformation|SetWorldTransform _item (Math|Transform|MakeTransform (.location _returnvalue) _output_get (.scale _returnvalue)) false false))

(event Input|EnhancedActionEvents|EnhancedInputActionIA_Interact
  (params (ActionValue :type Boolean) (ElapsedSeconds :type Float%20%28double-precision%29) (TriggeredSeconds :type Float%20%28double-precision%29) (InputAction :type Input%20Action%20Object%20Reference :default "/Game/Input/Actions/IA_Interact.IA_Interact"))
  (bind _returnvalue (Game|GetPlayerController 0))
  (:Started
    (Input|DisableInput _returnvalue)
    (Input|EnableInput (Variables|Default|GetCharacter) _returnvalue)
    (Utilities|IsValid (Variables|Default|GetWBP%20Ref)
      (:Is%20Valid
        (Widget|RemovefromParent (Variables|Default|GetWBP%20Ref))
        (Variables|Default|SetWBP%20Ref 0)
        (Actor|DestroyActor)))))

(event Input|EnhancedActionEvents|EnhancedInputActionIA_Move
  (params (ActionValue :type Vector%202D%20Structure) (ElapsedSeconds :type Float%20%28double-precision%29) (TriggeredSeconds :type Float%20%28double-precision%29) (InputAction :type Input%20Action%20Object%20Reference :default "/Game/Input/Actions/IA_Move.IA_Move"))
  ;[0.15 0.15 0.15 0.5] Move with WASD
  (if (or (!= (.x ActionValue) 0.0) (!= (.y ActionValue) 0.0))
    (Utilities|FlowControl|Sequence
      (:then_0
        (Transformation|SetWorldRotation (Variables|Default|GetItem) (Math|Rotator|CombineRotators (Transformation|GetWorldRotation (Variables|Default|GetItem)) (Math|Rotator|MakeRotator 0.0 0.0 (* (.x ActionValue) (Variables|Settings|UI|GetMove%20Speed)))) false false))
      (:then_1
        (Transformation|SetWorldRotation (Variables|Default|GetItem) (Math|Rotator|CombineRotators (Transformation|GetWorldRotation (Variables|Default|GetItem)) (Math|Rotator|MakeRotator 0.0 (* (.y ActionValue) (Variables|Settings|UI|GetMove%20Speed)) 0.0)) false false)))))

(event EventInspect
  (params (Character :type BP%20First%20Person%20Character%20Object%20Reference) (Inspected%20Item :type Static%20Mesh%20Object%20Reference) (Item%20Name :type Text) (Item%20Description :type Text))
  (bind _returnvalue (Game|GetPlayerController 0))
  (Variables|Default|SetCharacter Character)
  (Components|StaticMesh|SetStaticMesh (Variables|Default|GetItem) Inspected%20Item)
  (bind _returnvalue_2 (UserInterface|CreateWidget "/Game/Blueprints/Interactables/WBP_Interact.WBP_Interact_C" 0 Item%20Name Item%20Description))
  (bind _output_get (Variables|Default|SetWBP%20Ref _returnvalue_2))
  (UserInterface|Viewport|AddtoViewport _output_get 0)
  (Input|DisableInput (Variables|Default|GetCharacter) _returnvalue)
  (Input|EnableInput _returnvalue)
  (Class|BPIUI|UpdateInspiration(Message) (Variables|Default|GetCharacter) (Variables|Inspiration|GetInspirationGained)))

(event Input|MouseEvents|MouseX
  (params (AxisValue :type Float%20%28single-precision%29))
  ;[0.15 0.15 0.15 0.5] Set Mouse Horz Movement
  (if (Variables|Default|GetRotate?)
    (Transformation|SetWorldRotation (Variables|Default|GetItem) (Math|Rotator|CombineRotators (Transformation|GetWorldRotation (Variables|Default|GetItem)) (Math|Rotator|MakeRotator 0.0 0.0 (* AxisValue (Variables|Settings|UI|GetRot%20Speed)))) false false)))

(event Input|MouseEvents|MouseY
  (params (AxisValue :type Float%20%28single-precision%29))
  ;[0.15 0.15 0.15 0.5] Set Mouse Vert Movement
  (if (Variables|Default|GetRotate?)
    (Transformation|SetWorldRotation (Variables|Default|GetItem) (Math|Rotator|CombineRotators (Transformation|GetWorldRotation (Variables|Default|GetItem)) (Math|Rotator|MakeRotator 0.0 (* AxisValue (Variables|Settings|UI|GetRot%20Speed)) 0.0)) false false)))

(event Input|MouseEvents|LeftMouseButton
  (params (Key :type Key%20Structure :default "None"))
  ;[0.15 0.15 0.15 0.5] Only allow Rotation when Left Clicking
  (:Pressed
    (Variables|Default|SetRotate? true))
  (:Released
    (Variables|Default|SetRotate? false)))

(event Input|MouseEvents|RightMouseButton
  (params (Key :type Key%20Structure :default "None"))
  ;[0.15 0.15 0.15 0.5] Reset Transform of Inspected Item
  (:Pressed
    (Transformation|SetWorldRotation (Variables|Default|GetItem) (Variables|Default|GetInitial%20Rotation) false false)
    (Variables|/Script/Engine.SceneCaptureComponent2D|SetFOVAngle (Variables|Default|GetSceneCaptureComponent2D) (Variables|Default|GetInitial%202D%20FOV))))

(event Input|MouseEvents|MouseWheelUp
  (params (Key :type Key%20Structure :default "None"))
  (bind _scenecapturecomponent2d (Variables|Default|GetSceneCaptureComponent2D))
  ;[0.15 0.15 0.15 0.5] Zoom In
  (:Pressed
    (Variables|/Script/Engine.SceneCaptureComponent2D|SetFOVAngle _scenecapturecomponent2d (Math|Float|Clamp(Float) (- (Variables|/Script/Engine.SceneCaptureComponent2D|GetFOVAngle _scenecapturecomponent2d) (Variables|Settings|UI|GetZoom%20Increment)) (Variables|Settings|UI|GetZoom%20Min) (Variables|Settings|UI|GetZoom%20Max)))))

(event Input|MouseEvents|MouseWheelDown
  (params (Key :type Key%20Structure :default "None"))
  (bind _scenecapturecomponent2d (Variables|Default|GetSceneCaptureComponent2D))
  ;[0.15 0.15 0.15 0.5] Zoom Out
  (:Pressed
    (Variables|/Script/Engine.SceneCaptureComponent2D|SetFOVAngle _scenecapturecomponent2d (Math|Float|Clamp(Float) (+ (Variables|/Script/Engine.SceneCaptureComponent2D|GetFOVAngle _scenecapturecomponent2d) (Variables|Settings|UI|GetZoom%20Increment)) (Variables|Settings|UI|GetZoom%20Min) (Variables|Settings|UI|GetZoom%20Max)))))

(fn ConstructionScript
  (Variables|Default|SetInitial%202D%20FOV (Variables|/Script/Engine.SceneCaptureComponent2D|GetFOVAngle (Variables|Default|GetSceneCaptureComponent2D)))
  (Transformation|SetRelativeLocation (Variables|Default|GetInteractIcon) (Math|Vector|MakeVector 0.0 0.0 (+ (.z (.Max (Components|StaticMesh|GetLocalBounds (Variables|Default|GetItem)))) (Variables|Settings|UI|GetIconOffset))) false false))