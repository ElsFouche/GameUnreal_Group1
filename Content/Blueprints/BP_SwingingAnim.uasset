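; Actor that gives its Arrow component a looping swing on the pitch axis, judging by the names a swinging container animation.
; On BeginPlay it randomly offsets the swing amplitude and starting pitch, then starts the SwingingContainer timeline at a random play rate, either forward or in reverse.
; Each timeline update scales the Rotation track by the amplitude and adds the starting pitch, so separate instances swing out of sync.
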(event EventBeginPlay
  (bind _swingingcontainer (Variables|Default|GetSwingingContainer))
  (Variables|Default|SetRotationAmount (+ (Variables|Default|GetRotationAmount) (Math|Random|RandomFloatinRange -1.0 1.0)))
  (Variables|Default|SetArrowStartRot (Math|Rotator|MakeRotator 0.0 (+ (.Pitch (Math|Rotator|BreakRotator (Variables|/Script/Engine.SceneComponent|GetRelativeRotation (Variables|Default|GetArrow)))) (Math|Random|RandomFloatinRange -5.0 5.0)) 0.0))
  (Components|Timeline|SetLooping _swingingcontainer true)
  (Components|Timeline|SetPlayRate _swingingcontainer (Math|Random|RandomFloatinRange 0.8 1.2))
  (if (Math|Random|RandomBool)
    (bind _rotation (Timeline|SwingingContainer PlayFromStart)
      (:Update
        (Transformation|SetRelativeRotation (Variables|Default|GetArrow) (Math|Rotator|MakeRotator 0.0 (+ (* _rotation (Variables|Default|GetRotationAmount)) (.pitch (Variables|Default|GetArrowStartRot))) 0.0) false false)))
    (else
      (Timeline|SwingingContainer ReverseFromEnd))))

(fn ConstructionScript)