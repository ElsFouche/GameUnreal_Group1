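; AC_Ability is an actor component that lets its owner cast a fireball, gated by a cooldown.
; CastFireball spawns BP_Fireball at an offset along the given rotation's forward vector, plays a cast sound, and holds OnCooldown true for a timed Delay.
; A WB_FBCooldown widget, created at BeginPlay, shows only during cooldown, with its progress updated each tick from elapsed game time.
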(event Custom|Cast%20Fireball
  (params (Rotation :type Rotator) (Location :type Vector) (Offset :type Float%20%28double-precision%29))
  (if (not (Variables|Cooldown|Private|GetOnCooldown))
    ;[0.15 0.15 0.15 0.5] Spawn Fireball
    (Game|SpawnActorfromClass "/Game/Blueprints/Fireball/BP_Fireball.BP_Fireball_C" (Math|Transform|MakeTransform (+ Location (* (Math|Vector|Normalize (Math|Rotator|GetRotationXVector Rotation)) Offset)) Rotation "1.000000,1.000000,1.000000") "Undefined" "MultiplyWithRoot" 0 0.6 0)
    ;[0.15 0.15 0.15 0.5] Sound
    (Audio|PlaySoundatLocation (Variables|Sound|GetCast%20Sound) (Transformation|GetActorLocation (Components|GetOwner)) "0, 0, 0" 1.0 1.0 (Variables|Sound|GetStart%20Time) "/USDCore/USDDefaultAttenuation.USDDefaultAttenuation" 0 0 0)
    ;[0.15 0.15 0.15 0.5] Handle Cooldown
    (Variables|Cooldown|Private|SetOnCooldown true)
    (Variables|Cooldown|Private|SetCDStart (Utilities|Time|GetGameTimeinSeconds))
    (Widget|SetVisibility (Variables|Private|GetWB) "Visible")
    (Utilities|FlowControl|Delay (Variables|Cooldown|Public|GetCooldownDuration))
    (Variables|Cooldown|Private|SetOnCooldown false)
    (Variables|Cooldown|Private|SetCDProgress 0.0)
    (Widget|SetVisibility (Variables|Private|GetWB) "Hidden")))

(event EventTick
  (params (DeltaSeconds :type Float%20%28single-precision%29))
  (CallFunction|UpdateCDProgress))

(event EventBeginPlay
  ;[0.15 0.15 0.15 0.5] Create Widget
  (bind _returnvalue (UserInterface|CreateWidget "/Game/Blueprints/Fireball/WB_FBCooldown.WB_FBCooldown_C" (Game|GetPlayerController 0)))
  (bind _output_get (Variables|Private|SetWB _returnvalue))
  (Widget|SetVisibility _output_get "Hidden")
  (UserInterface|Viewport|AddtoViewport _output_get 0))

(fn UpdateCDProgress
  (bind _wb (Variables|Private|GetWB))
  (if (Variables|Cooldown|Private|GetOnCooldown)
    (bind _output_get (Variables|Cooldown|Private|SetCDProgress (/ (- (Utilities|Time|GetGameTimeinSeconds) (Variables|Cooldown|Private|GetCDStart)) (Variables|Cooldown|Public|GetCooldownDuration))))
    (Utilities|IsValid _wb
      (:Is%20Valid
        (Variables|/Game/Blueprints/Fireball/WB_FBCooldown.WB_FBCooldown_C|SetProgress _wb _output_get)))))