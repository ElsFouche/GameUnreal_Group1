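; Fireball actor that plays a blaze sound on spawn and destroys itself on hit.
; Targets implementing BPI_Damageable receive a damage message and a short-lived Chaos master field at their location, scaled by ImpactRadius and driven by Power.
; The explosion sound is handed to a spawned BP_SFXPlayer before the fireball is destroyed.
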(event Collision|EventHit
  (params (MyComp :type Primitive%20Component%20Object%20Reference) (Other :type Actor%20Object%20Reference) (OtherComp :type Primitive%20Component%20Object%20Reference) (bSelfMoved :type Boolean) (HitLocation :type Vector :default "0, 0, 0") (HitNormal :type Vector :default "0, 0, 0") (NormalImpulse :type Vector :default "0, 0, 0") (Hit :type Hit%20Result%20Structure%20%28by%20ref%29))
  (CallFunction|ApplyDamage Other)
  (Game|SpawnActorfromClass "/Game/Blueprints/BP_SFXPlayer.BP_SFXPlayer_C" (Math|Transform|MakeTransform (Transformation|GetActorLocation)) "Undefined" "MultiplyWithRoot" 0 (Variables|Default|GetExplosion%20SFX) (Variables|Default|GetExplosion%20Volume) 0.0 0)
  (Actor|DestroyActor))

(event EventBeginPlay
  (Audio|Components|Audio|Play (Variables|Default|GetSFX_Blaze) (Variables|Default|GetBlaze%20Start%20Time)))

(fn ConstructionScript)

(fn ApplyDamage
  (params (Other :type Actor%20Object%20Reference))
  (bind _returnvalue (Transformation|GetActorTransform Other))
  ;[0.15 0.15 0.15 0.5] Check if has Interface
  (if (Utilities|DoesObjectImplementInterface Other "/Game/Blueprints/Interfaces/BPI_Damageable.BPI_Damageable_C")
    (Class|BPIDamageable|ApplyDamage(Message) Other)
    ;[0.15 0.15 0.15 0.5] Spawn Field to Apply Damage
    (bind _returnvalue_2 (Game|SpawnActorfromClass "/Engine/EditorResources/FieldNodes/FS_MasterField.FS_MasterField_C" (Math|Transform|MakeTransform (.location _returnvalue) (.rotation _returnvalue) (* "1.000000,1.000000,1.000000" (Variables|Damage|GetImpactRadius))) "Undefined" "MultiplyWithRoot" 0 0))
    (bind _output_get (Variables|Damage|SetChaos%20Field _returnvalue_2))
    (Variables|/Engine/EditorResources/FieldNodes/FS_MasterField.FS_MasterField_C|SetRadial%20Magnitude _output_get (Variables|Damage|GetPower))
    (Variables|/Engine/EditorResources/FieldNodes/FS_MasterField.FS_MasterField_C|SetFieldLifespan _output_get 0.1)
    (Variables|/Engine/EditorResources/FieldNodes/FS_MasterField.FS_MasterField_C|SetActivationType _output_get "NewEnumerator4")
    (Actor|SetLifeSpan _output_get 0.1)
    (Default|CETrigger _output_get)))