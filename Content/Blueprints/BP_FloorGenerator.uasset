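; BP_FloorGenerator procedurally fills a grid with randomly chosen actors to build a floor, leaving random gaps.
; GenerateFloor clears earlier spawns, blocking-loads candidates from soft references, then spawns copies spaced by the previous pick's bounds and padding, with optional rotation and random scale.
; Each spawn receives a randomized chain length through an interface message.
; The construction script only runs Cleanup, destroying tracked spawned actors.
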(event EventGenerateFloor
  (bind _extents (Variables|ProcGen|GetExtents))
  (bind _actorsoftpath (Variables|ProcGen|GetActorSoftPath))
  (bind _padding (Variables|ProcGen|GetPadding))
  (bind _rotation (Variables|ProcGen|GetRotation))
  (bind _randomscale (Variables|ProcGen|GetRandomScale))
  (bind _possibleactors (Variables|ProcGen|GetPossibleActors))
  (bind (_x _y) (Utilities|Struct|BreakIntVector2 _extents))
  (bind (_x_2 _y_2) (Utilities|Struct|BreakIntVector2 _padding))
  (bind (_x_3 _y_3 _z) (Math|Vector|BreakVector _randomscale))
  (bind _returnvalue (* _randomscale -1))
  (if (Variables|ProcGen|GetbGenerationEnabled)
    (CallFunction|Cleanup)
    (if (Utilities|Array|IsEmpty _possibleactors)
      _
      (else
        (Utilities|Array|Clear _possibleactors)))
    (if (Utilities|Array|IsNotEmpty _actorsoftpath)
      (for _array_element _actorsoftpath
        (if (Utilities|IsValidSoftObjectReference _array_element)
          (bind _returnvalue_2 (Utilities|LoadAssetBlocking _array_element))
          (bind _asactor (Utilities|Casting|CastToActor _returnvalue_2)
            (:then
              (Utilities|Array|AddUnique (Variables|ProcGen|GetPossibleActors) _asactor))
            (:CastFailed
              (Development|PrintString "Cast to actor failed")))))
      (for _index (range 0 (- _y 1))
        (for _index_2 (range 0 (- _x 1))
          (Variables|ProcGen|SetPrevBoxExtent (.BoxExtent (Collision|GetActorBounds (Variables|ProcGen|GetTempActor) false true)))
          (Variables|ProcGen|SetTempActor (.OutItem (Utilities|Array|Random (Variables|ProcGen|GetPossibleActors))))
          (if (>= (Math|Random|RandomInteger 101) (Variables|ProcGen|GetGapChance))
            (bind _returnvalue_3 (Game|SpawnActorfromClass (Utilities|GetClass (Variables|ProcGen|GetTempActor)) (Math|Transform|MakeTransform (+ (Transformation|GetActorLocation) (* (Variables|ProcGen|GetPrevBoxExtent) (Math|Vector|MakeVector (Math|Conversions|ToFloat(Integer) _index_2) (Math|Conversions|ToFloat(Integer) _index) 0.0) (Math|Vector|MakeVector (/ (Math|Conversions|ToFloat(Integer) _x_2) 1e+02) (/ (Math|Conversions|ToFloat(Integer) _y_2) 1e+02) 0.0))) (Math|Rotator|SelectRotator (Transformation|GetActorRotation (Variables|ProcGen|GetTempActor)) _rotation (Utilities|Operators|EqualEqual :A _rotation)) (Math|Vector|SelectVector "1.000000,1.000000,1.000000" (Math|Vector|MakeVector (Math|Random|RandomFloatinRange (.x _returnvalue) _x_3) (Math|Random|RandomFloatinRange (.y _returnvalue) _y_3) (Math|Random|RandomFloatinRange (.z _returnvalue) _z)) (Utilities|Operators|EqualEqual :A _randomscale :ErrorTolerance 0.001))) "AdjustIfPossibleButAlwaysSpawn" "MultiplyWithRoot" 0 0))
            (Utilities|Array|Add (Variables|ProcGen|GetSpawnedActors) _returnvalue_3)
            (Class|BPIProcGen|IntParamFunc1(Message) _returnvalue_3 (+ (Variables|ProcGen|GetGenerateChains) (Math|Random|RandomIntegerinRange (* (Variables|ProcGen|GetRandomChainLength) -1) (Variables|ProcGen|GetRandomChainLength))))))))))

(event EventCleanup
  (bind _spawnedactors (Variables|ProcGen|GetSpawnedActors))
  (for _array_element _spawnedactors
    (Actor|DestroyActor _array_element))
  (Utilities|Array|Clear _spawnedactors))

(fn ConstructionScript
  (CallFunction|Cleanup))