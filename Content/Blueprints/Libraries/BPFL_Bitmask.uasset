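; Blueprint function library that treats an integer bitmask as a set of enum values, each mapped to bit 2^value.
; Add, remove and clear edit the mask by reference, alongside contains, empty, union, intersection and difference operations.
; ToArray extracts set bit indices by repeated halving, and Length counts that array.
; Remove's return value tests the raw enum integer rather than its power-of-two bit.
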(fn Add
  (params (Bitmask :type Integer%20%28by%20ref%29) (Enum :type Byte))
  (|SetBy-RefVar Bitmask (Class|KismetMathLibrary|OrIntInt Bitmask (CallFunction|PowerOfTwo (Math|Conversions|ToInteger(Byte) Enum))))
  (return))

(fn AddItems
  (params (Bitmask :type Integer%20%28by%20ref%29) (Enums :type Array%20of%20Bytes))
  (LocalVariables|SetSumOfEnums 0)
  (bind _arrayelement (Utilities|ForEachLoopReal Enums :!label _label)
    (:LoopBody
      (LocalVariables|SetSumOfEnums (Class|KismetMathLibrary|OrIntInt (CallFunction|PowerOfTwo (Math|Conversions|ToInteger(Byte) _arrayelement)) (LocalVariables|GetSumOfEnums)))
      (goto _label Continue))
    (:Completed
      (|SetBy-RefVar Bitmask (Class|KismetMathLibrary|OrIntInt Bitmask (LocalVariables|GetSumOfEnums)))
      (return))))

(fn Clear
  (params (Bitmask :type Integer%20%28by%20ref%29))
  (|SetBy-RefVar Bitmask))

(fn ContainsEnum
  (params (Bitmask :type Integer) (Enum :type Byte))
  (return (!= (Class|KismetMathLibrary|AndIntInt Bitmask (CallFunction|PowerOfTwo (Math|Conversions|ToInteger(Byte) Enum))) 0)))

(fn Difference
  (params (Bitmask1 :type Integer) (Bitmask2 :type Integer))
  (return (Class|KismetMathLibrary|AndIntInt Bitmask1 (Class|KismetMathLibrary|NotInt Bitmask2))))

(fn Intersection
  (params (Bitmask1 :type Integer) (Bitmaks2 :type Integer))
  (return (Class|KismetMathLibrary|AndIntInt Bitmask1 Bitmaks2)))

(fn IsEmpty
  (params (NewParam :type Integer))
  (return (== NewParam 0)))

(fn IsNotEmpty
  (params (Bitmask :type Integer))
  (return (!= Bitmask 0)))

(fn Length
  (params (Bitmask :type Integer))
  (bind _enums (Bitmask|ToArray Bitmask))
  (return (Utilities|Array|Length _enums)))

(fn Remove
  (params (Bitmask :type Integer%20%28by%20ref%29) (Enum :type Byte))
  (bind _returnvalue (Math|Conversions|ToInteger(Byte) Enum))
  (bind _output_get (LocalVariables|SetReturnValue (!= (Class|KismetMathLibrary|AndIntInt Bitmask _returnvalue) 0)))
  (|SetBy-RefVar Bitmask (Class|KismetMathLibrary|AndIntInt Bitmask (Class|KismetMathLibrary|NotInt (CallFunction|PowerOfTwo _returnvalue))))
  (return _output_get))

(fn RemoveItems
  (params (Bitmask :type Integer%20%28by%20ref%29) (Enums :type Array%20of%20Bytes))
  (LocalVariables|SetSumOfEnums 0)
  (bind _arrayelement (Utilities|ForEachLoopReal Enums :!label _label)
    (:LoopBody
      (LocalVariables|SetSumOfEnums (Class|KismetMathLibrary|OrIntInt (CallFunction|PowerOfTwo (Math|Conversions|ToInteger(Byte) _arrayelement)) (LocalVariables|GetSumOfEnums)))
      (goto _label Continue))
    (:Completed
      (|SetBy-RefVar Bitmask (Class|KismetMathLibrary|AndIntInt Bitmask (Class|KismetMathLibrary|NotInt (LocalVariables|GetSumOfEnums))))
      (return))))

(fn ToArray
  (params (Bitmask :type Integer))
  (LocalVariables|SetLocalBitmask Bitmask)
  (Utilities|Array|Clear (LocalVariables|GetTrueValues))
  (LocalVariables|SetAccumulator 0)
  (if (> (LocalVariables|GetLocalBitmask) 0) :!label _label
    (if (== (Utilities|Int% (LocalVariables|GetLocalBitmask) 2) 0)
      _
      (else
        (Utilities|Array|AddUnique (LocalVariables|GetTrueValues) (LocalVariables|GetAccumulator))))
    (LocalVariables|SetAccumulator (+ (LocalVariables|GetAccumulator) 1))
    (LocalVariables|SetLocalBitmask (/ (LocalVariables|GetLocalBitmask) 2))
    (goto _label)
    (else
      (return (LocalVariables|GetTrueValues)))))

(fn Union
  (params (Bitmask1 :type Integer) (Bitmask2 :type Integer))
  (return (Class|KismetMathLibrary|OrIntInt Bitmask1 Bitmask2)))