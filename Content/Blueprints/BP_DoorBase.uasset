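; Base door Blueprint that swings open when player 0's pawn enters its trigger and closes when it leaves.
; A timeline rotates the Arrow component's yaw 90 degrees from its starting value, playing forward to open and in reverse to close.
; A 2D dot product against the root's right vector picks the swing direction from the player's side.
; A DoOnce gates the opening sound until the timeline finishes, while a timeline event plays the quieter closing sound.
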(event OnComponentBeginOverlap(Trigger)
  (params (OverlappedComponent :type Primitive%20Component%20Object%20Reference) (OtherActor :type Actor%20Object%20Reference) (OtherComp :type Primitive%20Component%20Object%20Reference) (OtherBodyIndex :type Integer) (bFromSweep :type Boolean) (SweepResult :type Hit%20Result%20Structure%20%28by%20ref%29))
  (bind _startzrotation (Variables|Default|GetStartZRotation))
  (if (== OtherActor (Game|Player|GetPlayerPawn 0))
    (Utilities|FlowControl|Sequence
      (:then_0
        (Variables|Default|SetbIsClosing false)
        (bind _bisinfront (CallFunction|GetActorSideOfDoor))
        (Variables|Default|SetbActorIsInFront _bisinfront)
        (bind _dooropentrack (Timeline|DoorOpenClose Play)
          (:Update
            (Transformation|SetRelativeRotation (Variables|Default|GetArrow) (Math|Rotator|MakeRotator 0.0 0.0 (Math|Float|Lerp _startzrotation (+ _startzrotation (Math|Float|SelectFloat 9e+01 -9e+01 (Variables|Default|GetbActorIsInFront))) _dooropentrack)) false false))
          (:Finished
            (goto _label Reset))
          (:PlayAudio
            (if (Variables|Default|GetbIsClosing)
              (Audio|PlaySoundatLocation 0 (Transformation|GetActorLocation) "0, 0, 0" 0.6 1.0 0.0 0 0 0 0)))))
      (:then_1
        (Utilities|FlowControl|DoOnce false :!label _label
          (:Completed
            (Audio|PlaySoundatLocation 0 (Transformation|GetActorLocation) "0, 0, 0" 0.5 1.0 0.0 0 0 0 0)))))))

(event OnComponentEndOverlap(Trigger)
  (params (OverlappedComponent :type Primitive%20Component%20Object%20Reference) (OtherActor :type Actor%20Object%20Reference) (OtherComp :type Primitive%20Component%20Object%20Reference) (OtherBodyIndex :type Integer))
  (bind _startzrotation (Variables|Default|GetStartZRotation))
  (if (== OtherActor (Game|Player|GetPlayerPawn 0))
    (Variables|Default|SetbIsClosing true)
    (bind _dooropentrack (Timeline|DoorOpenClose Reverse)
      (:Update
        (Transformation|SetRelativeRotation (Variables|Default|GetArrow) (Math|Rotator|MakeRotator 0.0 0.0 (Math|Float|Lerp _startzrotation (+ _startzrotation (Math|Float|SelectFloat 9e+01 -9e+01 (Variables|Default|GetbActorIsInFront))) _dooropentrack)) false false))
      (:Finished
        (Utilities|FlowControl|DoOnce false) ; enters at Reset
      )
      (:PlayAudio
        (if (Variables|Default|GetbIsClosing)
          (Audio|PlaySoundatLocation 0 (Transformation|GetActorLocation) "0, 0, 0" 0.6 1.0 0.0 0 0 0 0))))))

(event EventBeginPlay
  (Variables|Default|SetStartZRotation (.yaw (Variables|/Script/Engine.SceneComponent|GetRelativeRotation (Variables|Default|GetArrow)))))

(fn ConstructionScript)

(fn GetActorSideOfDoor
  (bind _defaultsceneroot (Variables|Default|GetDefaultSceneRoot))
  (return (> (Math|Vector|DotProduct (- (Class|KismetMathLibrary|VectorNormal2D (Transformation|GetWorldLocation _defaultsceneroot) 0.0001) (Class|KismetMathLibrary|VectorNormal2D (Transformation|GetActorLocation (Game|Player|GetPlayerPawn 0)) 0.0001)) (Class|KismetMathLibrary|VectorNormal2D (Math|Vector|GetRightVector _defaultsceneroot) 0.0001)) 0.0)))