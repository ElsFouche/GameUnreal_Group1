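; Main game state Blueprint that manages three layered background music tracks.
; BeginPlay spawns danger, ambient and drum layers that persist across level transitions, and starts a looping timeline meant to modulate the drum layer's volume.
; RequestPlayBGM uses its priority argument both to pick a layer and to check against that layer's stored priority, which is never raised, then swaps the sound with a short fade out and in.
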(event EventBeginPlay
  (bind _fadeloops (Variables|Default|GetFadeLoops))
  (Components|Timeline|SetLooping _fadeloops true)
  (Audio|Components|Audio|Play _fadeloops)
  (bind _returnvalue (Audio|SpawnSound2D "/Game/Audio/BGM/BGM_NearDanger.BGM_NearDanger" 0.3 1.0 0.0 0 true false))
  (bind _output_get (Variables|Default|SetAudioLayer0 _returnvalue))
  (Utilities|Map|Add (Variables|Default|GetPriority) _output_get 0)
  (bind _returnvalue_2 (Audio|SpawnSound2D "/Game/Audio/BGM/BGM_HangDrumAmbient.BGM_HangDrumAmbient" 0.75 1.0 0.0 0 true false))
  (bind _output_get_2 (Variables|Default|SetAudioLayer1 _returnvalue_2))
  (Utilities|Map|Add (Variables|Default|GetPriority) _output_get_2 0)
  (bind _returnvalue_3 (Audio|SpawnSound2D "/Game/Audio/BGM/BGM_BodhanDrum.BGM_BodhanDrum" 1.0 1.0 0.0 0 true false))
  (bind _output_get_3 (Variables|Default|SetAudioLayer2 _returnvalue_3))
  (Utilities|Map|Add (Variables|Default|GetPriority) _output_get_3 0))

(event EventRequestPlayBGM
  (params (NewBGM :type Sound%20Wave%20Object%20Reference%20%28by%20ref%29) (StartTime :type Float%20%28double-precision%29) (Priority :type Integer) (Layer :type Integer))
  (bind _audiolayer0 (Variables|Default|GetAudioLayer0))
  (bind _audiolayer1 (Variables|Default|GetAudioLayer1))
  (bind _audiolayer2 (Variables|Default|GetAudioLayer2))
  (bind _returnvalue (Utilities|Select :Index Priority :Option%200 _audiolayer0 :Option%201 _audiolayer1 :Option%202 _audiolayer2))
  (if (<= (.Value (Utilities|Map|Find (Variables|Default|GetPriority) _returnvalue)) Priority)
    (Audio|Components|Audio|FadeOut _returnvalue 0.3 0.0 "Linear" :!class /Script/Engine.AudioComponent)
    (Utilities|FlowControl|Delay 0.3)
    (Audio|Components|Audio|SetSound _returnvalue NewBGM)
    (Audio|Components|Audio|FadeIn _returnvalue 0.3 1.0 0.0 "Linear" :!class /Script/Engine.AudioComponent)))

(fn ConstructionScript)